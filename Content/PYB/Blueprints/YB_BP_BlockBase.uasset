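; Base block actor for what appears to be a bird-launching destruction game, with configurable mesh, material and scale applied in the construction script.
; BeginPlay sets the default break threshold after a short delay.
; Hit only prints a debug string for Base_Bird impacts.
; The destruction logic, comparing impulse over mass to per-source thresholds before disabling collision and expiring the block, is disconnected and never runs.
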(event `self.StaticMesh.OnComponentBeginOverlap`
  (params (OverlappedComponent :type "PrimitiveComponent Object Reference") (OtherActor :type "Actor Object Reference") (OtherComp :type "PrimitiveComponent Object Reference") (OtherBodyIndex :type Integer) (bFromSweep :type Boolean) (SweepResult :type "HitResult Structure (by ref)")))

(event `self.ReceiveBeginPlay`
  (`KismetSystemLibrary.Delay` 1.0)
  (set `self.DefaultThreshold` 100.0))

(event `self.ReceiveTick`
  (params (DeltaSeconds :type "Float (single-precision)")))

(event `self.ReceiveHit`
  (params (MyComp :type "PrimitiveComponent Object Reference") (Other :type "Actor Object Reference") (OtherComp :type "PrimitiveComponent Object Reference") (bSelfMoved :type Boolean) (HitLocation :type "Vector Structure") (HitNormal :type "Vector Structure") (NormalImpulse :type "Vector Structure") (Hit :type "HitResult Structure (by ref)"))
  (cast `Base_Bird` Other)
  (`KismetSystemLibrary.PrintString` "Hello"))

(fn `UserConstructionScript`
  (`StaticMeshComponent.SetStaticMesh` (`self.StaticMesh`) (`self.BlockMesh`))
  (`PrimitiveComponent.SetMaterial` (`self.StaticMesh`) 0 (`self.BlockMat`))
  (`self.SetActorScale3D` (`KismetMathLibrary.MakeVector` (`self.ScaleX`) (`self.ScaleY`) (`self.ScaleZ`))))