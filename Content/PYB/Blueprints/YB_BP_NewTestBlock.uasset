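; Test block actor that falls until it finds ground, then rests on top of it.
; Each Tick, CheckGround traces down on the Visibility channel from the actor to just below the Box extent, with debug drawing on.
; Without a hit, the block moves vertically at a constant Gravity rate, with no acceleration.
; On the first hit, NewFunction snaps it onto the impact point, and NewVar prevents repeat snapping until ground is lost.
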(event `self.ReceiveTick`
  (params (DeltaSeconds :type "Float (single-precision)"))
  (bind _newparam (`self.CheckGround`))
  (if (`GameplayStatics.BreakHitResult` _newparam)
    (if (not (`self.NewVar`))
      (`self.NewFunction` _newparam)
      (set `self.NewVar` true))
    (else
      (`self.K2_AddActorWorldOffset` (`KismetMathLibrary.MakeVector` 0.0 0.0 (* DeltaSeconds (`self.gravity`))))
      (set `self.NewVar` false))))

(fn `CheckGround`
  (returns (NewParam :type "HitResult Structure"))
  (bind _returnvalue (`self.K2_GetActorLocation`))
  (bind (_returnvalue_x _returnvalue_y _returnvalue_z) (`KismetMathLibrary.BreakVector` (+ (`BoxComponent.BoxExtent` (`self.Box`)) (0.0 0.0 5.0))))
  (bind _outhit (`KismetSystemLibrary.LineTraceSingle` :`Start` _returnvalue :`End` (- _returnvalue (`KismetMathLibrary.MakeVector` 0.0 0.0 _returnvalue_z)) :`TraceChannel` "TraceTypeQuery1" :`DrawDebugType` "ForDuration"))
  (return _outhit))

(fn `NewFunction`
  (params (NewParam :type "HitResult Structure"))
  (bind (_boxextent_x _boxextent_y _boxextent_z) (`KismetMathLibrary.BreakVector` (`BoxComponent.BoxExtent` (`self.Box`))))
  (`self.K2_SetActorLocation` (+ (`.ImpactPoint` (`GameplayStatics.BreakHitResult` NewParam)) (`KismetMathLibrary.MakeVector` 0.0 0.0 _boxextent_z))))

(fn `UserConstructionScript`)