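; TNT block that explodes on hard enough impacts, then removes itself through a very short lifespan.
; Hits from actors with "Bird" in their class name compare raw impulse to a bird threshold.
; Other hits count only on sufficiently non-vertical normals, comparing impulse divided by the block's mass to a default threshold.
; That default threshold is assigned after a short delay at BeginPlay.
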(event `self.ReceiveBeginPlay`
  (`KismetSystemLibrary.Delay` 1.0)
  (set `self.DefaultThreshold` 100.0))

(event `self.ReceiveHit`
  (params (MyComp :type "PrimitiveComponent Object Reference") (Other :type "Actor Object Reference") (OtherComp :type "PrimitiveComponent Object Reference") (bSelfMoved :type Boolean) (HitLocation :type "Vector Structure") (HitNormal :type "Vector Structure") (NormalImpulse :type "Vector Structure") (Hit :type "HitResult Structure (by ref)"))
  (bind _returnvalue (`KismetMathLibrary.VSize` NormalImpulse))
  (if (`KismetStringLibrary.Contains` (`KismetSystemLibrary.GetClassDisplayName` (`GameplayStatics.GetObjectClass` Other)) "Bird")
    (if (> _returnvalue (`self.BirdThreshold`))
      (`self.Explode` :!label _label)
      (`self.SetLifeSpan` 0.01))
    (elif (< (`KismetMathLibrary.Abs` (`KismetMathLibrary.Dot_VectorVector` HitNormal (0.0 0.0 1.0))) 0.8)
      (if (> (/ _returnvalue (`PrimitiveComponent.GetMass` (`self.StaticMesh`))) (`self.DefaultThreshold`))
        (goto _label)))))

(fn `UserConstructionScript`)